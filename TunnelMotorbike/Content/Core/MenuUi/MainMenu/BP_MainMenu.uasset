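; BP_MainMenu is an actor that sets up the main menu and its high score board on BeginPlay.
; It first calls LoadGameData on BP_GameInstance, then creates WBP_MainMenu and adds it to the viewport.
; The platform name picks the widget switcher page and cursor visibility: Windows shows the cursor, while Android and iOS share a cursorless page.
; Finally, it reads the high score field from the saved JSON and passes it to the widget.
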(event EventBeginPlay
  ;[0 0 0 0.5] Create the widegt of main menu when begin
  (Utilities|FlowControl|Sequence
    (:then_0
      (Default|LoadGameData (.AsBP%20Game%20Instance (Utilities|Casting|CastToBP_GameInstance (Game|GetGameInstance))) false))
    (:then_1
      (bind _returnvalue (UserInterface|CreateWidget "/Game/Core/MenuUi/MainMenu/WBP_MainMenu.WBP_MainMenu_C"))
      (Variables|Default|SetCreatedMainMenu _returnvalue)
      (switch string (Game|GetPlatformName)
        (:Windows
          (Class|WidgetSwitcher|SetActiveWidgetIndex (Variables|/Game/Core/MenuUi/MainMenu/WBP_MainMenu.WBP_MainMenu_C|GetWidgetSwitcher_MainMenu (Variables|Default|GetCreatedMainMenu)))
          (UserInterface|Viewport|AddtoViewport (Variables|Default|GetCreatedMainMenu) 0)
          (Variables|/Script/Engine.PlayerController|SetbShowMouseCursor (Game|GetPlayerController 0) true))
        (:Android
          (Class|WidgetSwitcher|SetActiveWidgetIndex (Variables|/Game/Core/MenuUi/MainMenu/WBP_MainMenu.WBP_MainMenu_C|GetWidgetSwitcher_MainMenu (Variables|Default|GetCreatedMainMenu)) 1 :!label _label)
          (UserInterface|Viewport|AddtoViewport (Variables|Default|GetCreatedMainMenu) 0)
          (Variables|/Script/Engine.PlayerController|SetbShowMouseCursor (Game|GetPlayerController 0) false))
        (:IOS
          (goto _label))))
    (:then_2
      ;[0.15 0.15 0.15 0.5] Comment
      (bind (_outvalue _returnvalue_2) (|GetJsonField (Variables|/Game/Core/SaveGame/BP_GameInstance.BP_GameInstance_C|GetSavedJsonData (.AsBP%20Game%20Instance (Utilities|Casting|CastToBP_GameInstance (Game|GetGameInstance)))) "HighScore Board Info"))
      (if _returnvalue_2
        (Variables|Default|SetHighScoreRecord _outvalue)
        (Utilities|IsValid (Variables|Default|GetCreatedMainMenu)
          (:Is%20Valid
            (Default|UpdateHighscoreDataBaseonPlatform (Variables|Default|GetCreatedMainMenu) (Variables|Default|GetHighScoreRecord))))))))

(fn ConstructionScript)