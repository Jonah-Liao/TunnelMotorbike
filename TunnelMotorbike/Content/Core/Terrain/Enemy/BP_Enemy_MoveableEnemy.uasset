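; Terrain enemy whose static mesh bobs vertically between zero and a maximum relative height, pausing at each end.
; A looping timer, started by a separate event rather than BeginPlay, drives each movement step and accumulates wait time, clamping the descent at zero.
; A random play rate varies speed per instance.
; The reset event clears the timer, restores the start position and upward state, and re-rolls the rate.
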(event Custom|StartMoveEnemyRelativeLocationForLoop
  (bind _returnvalue (Utilities|Time|SetTimerbyEvent (delegate Custom|MoveEnemyRelativeLocation) (Variables|Default|GetDeltaTime) true))
  (Variables|Default|SetTimer_RelativeLocationMove _returnvalue))

(event Custom|StopEnemyRelationLocationMovementAndResetState
  (CallFunction|StopandClearEnemyMovementTimer)
  (Transformation|SetRelativeLocation (Variables|Default|GetStaticMesh_Enemy) (Variables|Default|GetStartRelativeLocation) false false)
  (Variables|Default|SetIsMoveUp true)
  (Variables|Default|SetIsStopMovement false)
  (Variables|Default|SetMovePlayRate (Math|Random|RandomFloatinRange 0.5 1.6)))

(event Custom|MoveEnemyRelativeLocation
  (bind _staticmesh_enemy (Variables|Default|GetStaticMesh_Enemy))
  (bind _relativelocation (Variables|/Script/Engine.SceneComponent|GetRelativeLocation _staticmesh_enemy))
  (bind _z (Math|Vector|BreakVector _relativelocation))
  (if (Variables|Default|GetIsStopMovement)
    (bind _output_get (Variables|Default|SetRecordedStopTime (+ (Variables|Default|GetRecordedStopTime) (Variables|Default|GetDeltaTime))))
    (if (>= _output_get (Variables|Default|GetWaitTimeBetweenMovement))
      (Variables|Default|SetIsStopMovement false)
      (Variables|Default|SetRecordedStopTime 0.0))
    (elif (Variables|Default|GetIsMoveUp)
      (if (>= (.z (Variables|/Script/Engine.SceneComponent|GetRelativeLocation (Variables|Default|GetStaticMesh_Enemy))) (.Z (Math|Vector|BreakVector (Variables|Default|GetMaxRelativeLocation))))
        (Variables|Default|SetIsMoveUp false)
        (Variables|Default|SetIsStopMovement true)
        (else
          (Transformation|AddRelativeLocation (Variables|Default|GetStaticMesh_Enemy) (Math|Vector|MakeVector 0.0 0.0 (* (Variables|Default|GetDeltaDistance) 1.0 (Variables|Default|GetMovePlayRate))) false false)))
      (elif (<= (.z (Variables|/Script/Engine.SceneComponent|GetRelativeLocation (Variables|Default|GetStaticMesh_Enemy))) 0.0)
        (Variables|Default|SetIsMoveUp true)
        (Variables|Default|SetIsStopMovement true)
        (else
          (Transformation|AddRelativeLocation (Variables|Default|GetStaticMesh_Enemy) (Math|Vector|MakeVector 0.0 0.0 (select (> (- _z (* (Variables|Default|GetDeltaDistance) (Variables|Default|GetMovePlayRate))) 0.0) (* (Variables|Default|GetDeltaDistance) -1.0 (Variables|Default|GetMovePlayRate)) (* _z -1.0))) false false))))))

(event Custom|StopAndClearEnemyMovementTimer
  (Utilities|Time|ClearandInvalidateTimerbyHandle (Variables|Default|GetTimer_RelativeLocationMove)))

(event EventBeginPlay
  (Variables|Default|SetMovePlayRate (Math|Random|RandomFloatinRange 0.8 1.6)))

(fn ConstructionScript
  (|CallParentFunction))