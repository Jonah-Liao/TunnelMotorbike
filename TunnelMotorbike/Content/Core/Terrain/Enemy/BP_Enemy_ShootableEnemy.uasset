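; Terrain enemy that watches for the player aircraft with a laser sight and fires a bullet after a short warning delay.
; While detection is enabled, a looping timer capsule-traces along world -X over a set number of grid cells, fitting the Niagara beam to any hit.
; Hitting BP_Pawn switches the laser color and starts a countdown, after which it spawns BP_EnemyShotBullet.
; A reset event hides the laser and stops detection.
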(event Custom|DetectPlayerAircraft
  (if (and (not (Variables|Default|GetIsCalculatingTimeBeforeShot)) (Variables|Default|GetIsShootable))
    (Effects|Components|ParticleSystem|SetColorParameter (Variables|Default|GetNiagara_Laser) "Color001" (Variables|Default|GetPlayerUndetectedColor))
    (Rendering|SetVisibility (Variables|Default|GetNiagara_Laser) true false)
    (Components|Activation|SetActive (Variables|Default|GetNiagara_Laser) true false)
    (bind (_outhit _returnvalue) (Collision|CapsuleTraceByChannel (Transformation|GetWorldLocation (Variables|Default|GetLineTraceStartPoint)) (+ (Transformation|GetWorldLocation (Variables|Default|GetLineTraceStartPoint)) (Math|Vector|MakeVector (* (.X (Math|Vector2D|BreakVector2D (Variables|/Game/Core/Terrain/BP_Terrain.BP_Terrain_C|GetGridSize (Variables|/Game/Core/CombatSystem/BP_CombatSystem.BP_CombatSystem_C|GetTerrain (Variables|Default|GetCombatSystem))))) (Variables|Default|GetLineTraceGridNum) -1.0) 0.0 0.0)) 3e+01 0.0 "TraceTypeQuery3" false 0 "None"))
    (if _returnvalue
      (Effects|Components|ParticleSystem|SetVectorParameter (Variables|Default|GetNiagara_Laser) "Beam End" (Math|Vector|MakeVector (.Distance (Collision|BreakHitResult _outhit)) 0.0 0.0))
      (Utilities|Casting|CastToBP_Pawn (.HitActor (Collision|BreakHitResult _outhit)))
      (Variables|Default|SetIsCalculatingTimeBeforeShot true)
      (Variables|Default|SetCurrentLeftTimeBeforeShot (Variables|Default|GetWaitTimeAfterDetectingPlayer))
      (Effects|Components|ParticleSystem|SetColorParameter (Variables|Default|GetNiagara_Laser) "Color001" (Variables|Default|GetPlayerDetectedColor))
      (else
        (Effects|Components|ParticleSystem|SetVectorParameter (Variables|Default|GetNiagara_Laser) "Beam End" (Math|Vector|MakeVector (* (.X (Math|Vector2D|BreakVector2D (Variables|/Game/Core/Terrain/BP_Terrain.BP_Terrain_C|GetGridSize (Variables|/Game/Core/CombatSystem/BP_CombatSystem.BP_CombatSystem_C|GetTerrain (Variables|Default|GetCombatSystem))))) (Variables|Default|GetLineTraceGridNum)) 0.0 0.0))))
    (else
      (bind _output_get (Variables|Default|SetCurrentLeftTimeBeforeShot (- (Variables|Default|GetCurrentLeftTimeBeforeShot) (Variables|Default|GetDeltaTime))))
      (if (<= _output_get 0.0)
        (CallFunction|ShotOutEnemyBullet)
        (Variables|Default|SetIsCalculatingTimeBeforeShot false)
        (Effects|Components|ParticleSystem|SetColorParameter (Variables|Default|GetNiagara_Laser) "Color001" (Variables|Default|GetPlayerUndetectedColor))
        (Components|Activation|SetActive (Variables|Default|GetNiagara_Laser) false false)))))

(event Custom|StopDetectPlayerAircraftAndReset
  (Rendering|SetVisibility (Variables|Default|GetNiagara_Laser) false false)
  (Components|Activation|SetActive (Variables|Default|GetNiagara_Laser) false false)
  (CallFunction|ClearLineTraceTimerandDisableShoot)
  (Variables|Default|SetIsCalculatingTimeBeforeShot false)
  (Variables|Default|SetCurrentLeftTimeBeforeShot 0.0))

(event Custom|StartDetectPlayer
  (Variables|Default|SetIsShootable true)
  (bind _returnvalue (Utilities|Time|SetTimerbyEvent (delegate Custom|DetectPlayerAircraft) (Variables|Default|GetDeltaTime) true))
  (Variables|Default|SetPlayerDetectLineChannelTimer _returnvalue))

(event Custom|ClearLineTraceTimerAndDisableShoot
  (Variables|Default|SetIsShootable false)
  (Utilities|Time|ClearandInvalidateTimerbyHandle (Variables|Default|GetPlayerDetectLineChannelTimer)))

(event EventBeginPlay
  (Rendering|SetVisibility (Variables|Default|GetNiagara_Laser) false false)
  (Components|Activation|SetActive (Variables|Default|GetNiagara_Laser) false false))

(fn ConstructionScript
  (|CallParentFunction))

(fn SetEnemyStaticMesh
  (|CallParentFunction))

(fn ShotOutEnemyBullet
  (bind _bulletshotoutpoint (Variables|Default|GetBulletShotOutPoint))
  (bind _returnvalue (Transformation|GetWorldTransform _bulletshotoutpoint))
  (if (Variables|Default|GetIsShootable)
    (bind _returnvalue_2 (Game|SpawnActorfromClass "/Game/Core/Terrain/Enemy/BP_EnemyShotBullet.BP_EnemyShotBullet_C" _returnvalue "Undefined" "MultiplyWithRoot" 0 (Variables|Default|GetCombatSystem) _returnvalue 0))
    (Variables|Default|SetEnemyBullet _returnvalue_2)))