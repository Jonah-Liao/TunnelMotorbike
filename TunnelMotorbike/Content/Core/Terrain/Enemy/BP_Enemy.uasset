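; BP_Enemy is a terrain enemy actor with a configurable static mesh and a colour drawn from the selectable colour enum.
; The construction script applies the mesh.
; BeginPlay creates and caches a dynamic material instance, then sets its GridColor to either a specified colour or a random enum entry.
; SetBasicData stores a reference to the combat system, which the actor's own graphs do not otherwise use.
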(event EventBeginPlay
  (CallFunction|UpdateEnemyDynamicMaterialandColor))

(event Collision|EventActorBeginOverlap
  (params (OtherActor :type Actor%20Object%20Reference)))

(event EventTick
  (params (DeltaSeconds :type Float%20%28single-precision%29)))

(fn ConstructionScript
  (CallFunction|SetEnemyStaticMesh))

(fn SetEnemyStaticMesh
  (Components|StaticMesh|SetStaticMesh (Variables|Default|GetStaticMesh_Enemy) (Variables|Default|GetSM_Enemy)))

(fn UpdateEnemyDynamicMaterialandColor
  (bind _staticmesh_enemy (Variables|Default|GetStaticMesh_Enemy))
  (Utilities|IsValid _staticmesh_enemy
    (:Is%20Valid
      (Utilities|IsValid (Variables|Default|GetCurrentDynamicMaterial)
        (:Is%20Valid
          _)
        (:Is%20Not%20Valid
          (bind _returnvalue (Rendering|Material|CreateDynamicMaterialInstance _staticmesh_enemy 0 "/Game/Asset/Material/MI_Enemy.MI_Enemy" "None" :!class /Script/Engine.PrimitiveComponent))
          (Variables|Default|SetCurrentDynamicMaterial _returnvalue)))
      (if (Variables|Default|GetIsUseSpecificColor)
        (Variables|Default|SetCurrentColor (Variables|Default|GetSpecificColor))
        (else
          (Variables|Default|SetCurrentColor (Utilities|Enum|ByteToEnumE_SelectableColor (Math|Conversions|ToByte(Integer) (Math|Random|RandomIntegerinRange 0 (- (|GetNumEnumEntries) 1)))))))
      (Rendering|Material|SetVectorParameterValue (Variables|Default|GetCurrentDynamicMaterial) "GridColor" (CallFunction|GetLinearColorbyColorType (Variables|Default|GetCurrentColor)) :!class /Script/Engine.MaterialInstanceDynamic))))

(fn SetBasicData
  (params (CurrentCombatSystem :type BP%20Combat%20System%20Object%20Reference))
  (Variables|Default|SetCombatSystem CurrentCombatSystem))