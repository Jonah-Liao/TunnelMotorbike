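; Enemy projectile that travels along negative X on the scrolling combat terrain and is destroyed when a player bullet overlaps it.
; A looping timer moves it by its speed plus the terrain's backward scroll, destroying it past a grid-based limit.
; CombatSystem events pause, resume or destroy it.
; Two collision components detect player bullets; overlapping the player pawn currently does nothing in this graph.
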(event OnComponentBeginOverlap(EnemyBulletCollision)
  (params (OverlappedComponent :type Primitive%20Component%20Object%20Reference) (OtherActor :type Actor%20Object%20Reference) (OtherComp :type Primitive%20Component%20Object%20Reference) (OtherBodyIndex :type Integer) (bFromSweep :type Boolean) (SweepResult :type Hit%20Result%20Structure%20%28by%20ref%29))
  (Utilities|Casting|CastToBP_Pawn OtherActor
    (:CastFailed
      (Utilities|Casting|CastToBP_PlayerBullet OtherActor)
      (Actor|DestroyActor))))

(event OnComponentBeginOverlap(EnemyBulletCollision_CheckPlayerBullet)
  (params (OverlappedComponent :type Primitive%20Component%20Object%20Reference) (OtherActor :type Actor%20Object%20Reference) (OtherComp :type Primitive%20Component%20Object%20Reference) (OtherBodyIndex :type Integer) (bFromSweep :type Boolean) (SweepResult :type Hit%20Result%20Structure%20%28by%20ref%29))
  (Utilities|Casting|CastToBP_PlayerBullet OtherActor)
  (Actor|DestroyActor))

(event Custom|MoveEnemyBulletTowardPlayerDirection
  (Transformation|SetActorLocation (Math|Vector|MakeVector (- (.X (Math|Vector|BreakVector (.Location (Math|Transform|BreakTransform (Variables|Default|GetCurrentBulletWorldTransform))))) (+ (Variables|/Game/Core/Terrain/BP_Terrain.BP_Terrain_C|GetCurrentBackwardDistancePerTime (Variables|/Game/Core/CombatSystem/BP_CombatSystem.BP_CombatSystem_C|GetTerrain (Variables|Default|GetCombatSystem))) (Variables|Default|GetEnemyBulletSpeed))) (.Y (Math|Vector|BreakVector (.Location (Math|Transform|BreakTransform (Variables|Default|GetCurrentBulletWorldTransform))))) (.Z (Math|Vector|BreakVector (.Location (Math|Transform|BreakTransform (Variables|Default|GetCurrentBulletWorldTransform)))))) false false)
  (bind _output_get (Variables|Default|SetCurrentBulletWorldTransform (Math|Transform|MakeTransform (Math|Vector|MakeVector (- (.X (Math|Vector|BreakVector (.Location (Math|Transform|BreakTransform (Variables|Default|GetCurrentBulletWorldTransform))))) (+ (Variables|/Game/Core/Terrain/BP_Terrain.BP_Terrain_C|GetCurrentBackwardDistancePerTime (Variables|/Game/Core/CombatSystem/BP_CombatSystem.BP_CombatSystem_C|GetTerrain (Variables|Default|GetCombatSystem))) (Variables|Default|GetEnemyBulletSpeed))) (.Y (Math|Vector|BreakVector (.Location (Math|Transform|BreakTransform (Variables|Default|GetCurrentBulletWorldTransform))))) (.Z (Math|Vector|BreakVector (.Location (Math|Transform|BreakTransform (Variables|Default|GetCurrentBulletWorldTransform)))))) (.Rotation (Math|Transform|BreakTransform (Variables|Default|GetCurrentBulletWorldTransform))) (.Scale (Math|Transform|BreakTransform (Variables|Default|GetCurrentBulletWorldTransform))))))
  (if (< (.X (Math|Vector|BreakVector (.Location (Math|Transform|BreakTransform _output_get)))) (* (.X (Math|Vector2D|BreakVector2D (Variables|/Game/Core/Terrain/BP_Terrain.BP_Terrain_C|GetGridSize (Variables|/Game/Core/CombatSystem/BP_CombatSystem.BP_CombatSystem_C|GetTerrain (Variables|Default|GetCombatSystem))))) (Variables|Default|GetDestroyWhenMoveAfterPlayerGridNum) -1.0))
    (Utilities|Time|ClearandInvalidateTimerbyHandle (Variables|Default|GetEnemyBulletMovingTimer))
    (Actor|DestroyActor)))

(event Custom|StartMovingEnemyBullet
  (bind _returnvalue (Utilities|Time|SetTimerbyEvent (delegate Custom|MoveEnemyBulletTowardPlayerDirection) 0.02 true))
  (Variables|Default|SetEnemyBulletMovingTimer _returnvalue))

(event Custom|OnCombatPaused
  (Utilities|Time|ClearandInvalidateTimerbyHandle (Variables|Default|GetEnemyBulletMovingTimer)))

(event Custom|OnCombatContinue
  (CallFunction|StartMovingEnemyBullet))

(event Custom|OnCombatEnd
  (Actor|DestroyActor))

(event EventBeginPlay
  (bind _combatsystem (Variables|Default|GetCombatSystem))
  (Utilities|FlowControl|Sequence
    (:then_0
      (EventDispatchers|BindEventtoOnCombatPaused _combatsystem (EventDispatchers|CreateEvent :!event Custom|OnCombatPaused))
      (EventDispatchers|BindEventtoOnCombatContinue _combatsystem (EventDispatchers|CreateEvent :!event Custom|OnCombatContinue))
      (EventDispatchers|BindEventtoOnCombatEnd _combatsystem (EventDispatchers|CreateEvent :!event Custom|OnCombatEnd)))
    (:then_1
      (Variables|Default|SetCurrentBulletWorldTransform (Variables|Default|GetBulletStartWorldTransform))
      (CallFunction|StartMovingEnemyBullet))))

(fn ConstructionScript)