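; BP_CollectableItem is a collectable item actor in the terrain system with a configurable mesh and a color type; it contains no pickup logic.
; The construction script applies the chosen mesh to its static mesh component.
; On BeginPlay it creates a dynamic material, if none exists, from an opaque or transparent source per blend type.
; It then sets the GridColor parameter from either a specified color or a random selectable color.
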(event EventBeginPlay
  (CallFunction|UpdateDynamicMaterialandColor))

(event Collision|EventActorBeginOverlap
  (params (OtherActor :type Actor%20Object%20Reference)))

(event EventTick
  (params (DeltaSeconds :type Float%20%28single-precision%29)))

(fn ConstructionScript
  (CallFunction|SetStaticMesh))

(fn SetStaticMesh
  (Components|StaticMesh|SetStaticMesh (Variables|Default|GetStaticMesh_CollectableItem) (Variables|Default|GetCollectableItemMesh)))

(fn UpdateDynamicMaterialandColor
  (bind _staticmesh_collectableitem (Variables|Default|GetStaticMesh_CollectableItem))
  (Utilities|IsValid (Variables|Default|GetStaticMesh_CollectableItem)
    (:Is%20Valid
      (Utilities|IsValid (Variables|Default|GetCurrentDynamicMaterial)
        (:Is%20Valid
          _)
        (:Is%20Not%20Valid
          (switch Utilities|FlowControl|Switch|SwitchonE_MaterialUsingType (Variables|Default|GetCurrentDynamicMaterialBlendType)
            (:NewEnumerator0
              (bind _returnvalue (Rendering|Material|CreateDynamicMaterialInstance _staticmesh_collectableitem 0 "/Game/Asset/Material/MI_GridCollectableItem.MI_GridCollectableItem" "None" :!class /Script/Engine.PrimitiveComponent))
              (Variables|Default|SetCurrentDynamicMaterial _returnvalue))
            (:NewEnumerator1
              (bind _returnvalue_2 (Rendering|Material|CreateDynamicMaterialInstance _staticmesh_collectableitem 0 "/Game/Asset/Material/MI_IncreaseSpeed_Transparent.MI_IncreaseSpeed_Transparent" "None" :!class /Script/Engine.PrimitiveComponent))
              (Variables|Default|SetCurrentDynamicMaterial _returnvalue_2)))))
      (if (Variables|Default|GetIsUseSpecificColor)
        (Variables|Default|SetCurrentColor (Variables|Default|GetSpecificColor))
        (else
          (Variables|Default|SetCurrentColor (Utilities|Enum|ByteToEnumE_SelectableColor (Math|Conversions|ToByte(Integer) (Math|Random|RandomIntegerinRange 0 (- (|GetNumEnumEntries) 1)))))))
      (Rendering|Material|SetVectorParameterValue (Variables|Default|GetCurrentDynamicMaterial) "GridColor" (CallFunction|GetLinearColorbyColorType (Variables|Default|GetCurrentColor)) :!class /Script/Engine.MaterialInstanceDynamic))))