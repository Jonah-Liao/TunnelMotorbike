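; BP_CollectableItem_Coin is a coin collectable item that can spin its static mesh.
; StartRotateCoinForLoop runs a looping timer that adds a relative rotation delta to the mesh at short intervals, instead of using Tick.
; StopCoinForLoop clears that timer through its stored handle.
; Nothing in this graph calls either event, overlap logic is empty, and construction defers to the parent.
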(event Custom|StartRotateCoinForLoop
  (bind _returnvalue (Utilities|Time|SetTimerbyEvent (delegate Custom|RotateCoinRelativeRotation) 0.1 true))
  (Variables|Default|SetTimer_CoinLoopingRotation _returnvalue))

(event Custom|StopCoinForLoop
  (Utilities|Time|ClearandInvalidateTimerbyHandle (Variables|Default|GetTimer_CoinLoopingRotation)))

(event Custom|RotateCoinRelativeRotation
  (Transformation|AddRelativeRotation (Variables|Default|GetStaticMesh_CollectableItem) (Variables|Default|GetCoinDeltaRotation) false false))

(event EventBeginPlay)

(event Collision|EventActorBeginOverlap
  (params (OtherActor :type Actor%20Object%20Reference)))

(event EventTick
  (params (DeltaSeconds :type Float%20%28single-precision%29)))

(fn ConstructionScript
  (|CallParentFunction))