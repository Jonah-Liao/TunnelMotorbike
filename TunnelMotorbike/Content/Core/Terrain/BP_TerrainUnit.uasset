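; Terrain grid unit that carries pre-placed child actors for three enemy types (stable, moving, shooting) and three pickups (bullet, coin, speed increase).
; BeginPlay caches the child actors and passes CombatSystem to the enemies.
; Show/Destroy functions pool them in place by toggling visibility, collision and spawn flags rather than spawning or destroying.
; They also start or stop coin rotation, enemy movement and player detection, and most Show calls record ItemColor.
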(event EventBeginPlay
  (Utilities|FlowControl|Sequence
    (:then_0
      (Variables|Default|SetCollectableItem_Bullet (.AsBP%20Collectable%20Item%20Bullet (Utilities|Casting|CastToBP_CollectableItem_Bullet (Variables|/Script/Engine.ChildActorComponent|GetChildActor (Variables|Default|GetChildActor_CollectableItem_Bullet)))))
      (Variables|Default|SetCollectableItem_Coin (.AsBP%20Collectable%20Item%20Coin (Utilities|Casting|CastToBP_CollectableItem_Coin (Variables|/Script/Engine.ChildActorComponent|GetChildActor (Variables|Default|GetChildActor_CollectableItem_Coin)))))
      (Variables|Default|SetCollectableItem_SpeedIncrease (.AsBP%20Collectable%20Item%20Speed%20Increase (Utilities|Casting|CastToBP_CollectableItem_SpeedIncrease (Variables|/Script/Engine.ChildActorComponent|GetChildActor (Variables|Default|GetChildActor_CollectableItem_SpeedIncrease))))))
    (:then_1
      (bind _output_get (Variables|Default|SetEnemy_StableObstacle (.AsBP%20Enemy (Utilities|Casting|CastToBP_Enemy (Variables|/Script/Engine.ChildActorComponent|GetChildActor (Variables|Default|GetChildActor_Enemy_Stable))))))
      (Default|SetBasicData _output_get (Variables|Default|GetCombatSystem))
      (bind _output_get_2 (Variables|Default|SetEnemy_MoveableEnemy (.AsBP%20Enemy%20Moveable%20Enemy (Utilities|Casting|CastToBP_Enemy_MoveableEnemy (Variables|/Script/Engine.ChildActorComponent|GetChildActor (Variables|Default|GetChildActor_Enemy_MoveType))))))
      (Default|SetBasicData _output_get_2 (Variables|Default|GetCombatSystem))
      (bind _output_get_3 (Variables|Default|SetEnemy_ShotableEnemy (.AsBP%20Enemy%20Shootable%20Enemy (Utilities|Casting|CastToBP_Enemy_ShootableEnemy (Variables|/Script/Engine.ChildActorComponent|GetChildActor (Variables|Default|GetChildActor_Enemy_ShotableType))))))
      (Default|SetBasicData _output_get_3 (Variables|Default|GetCombatSystem)))))

(fn ConstructionScript)

(fn ShowObstacleonGrid
  (bind _enemy_stableobstacle (Variables|Default|GetEnemy_StableObstacle))
  (bind _enemy_stableobstacle_2 (Variables|Default|GetEnemy_StableObstacle))
  (bind _enemy_stableobstacle_3 (Variables|Default|GetEnemy_StableObstacle))
  (bind _staticmesh_enemy (Variables|/Game/Core/Terrain/Enemy/BP_Enemy.BP_Enemy_C|GetStaticMesh_Enemy _enemy_stableobstacle_2))
  (bind _staticmesh_enemy_2 (Variables|/Game/Core/Terrain/Enemy/BP_Enemy.BP_Enemy_C|GetStaticMesh_Enemy _enemy_stableobstacle_3))
  (Variables|Default|SetIsSpawnObstacle true)
  (Rendering|SetVisibility _staticmesh_enemy true false)
  (Development|SetHiddeninGame _staticmesh_enemy false false)
  (Collision|SetCollisionEnabled _staticmesh_enemy_2 "QueryOnly")
  (Collision|SetCollisionResponsetoChannel _staticmesh_enemy_2 "ECC_Pawn" "ECR_Overlap")
  (Collision|SetCollisionResponsetoChannel _staticmesh_enemy_2 "ECC_GameTraceChannel2" "ECR_Overlap")
  (Collision|SetCollisionResponsetoChannel _staticmesh_enemy_2 "ECC_GameTraceChannel6" "ECR_Block")
  (Default|UpdateEnemyDynamicMaterialandColor _enemy_stableobstacle)
  (Variables|Default|SetItemColor (Variables|/Game/Core/Terrain/Enemy/BP_Enemy.BP_Enemy_C|GetCurrentColor _enemy_stableobstacle)))

(fn DestroyObstacleonGrid
  (bind _enemy_stableobstacle (Variables|Default|GetEnemy_StableObstacle))
  (bind _enemy_stableobstacle_2 (Variables|Default|GetEnemy_StableObstacle))
  (bind _staticmesh_enemy (Variables|/Game/Core/Terrain/Enemy/BP_Enemy.BP_Enemy_C|GetStaticMesh_Enemy _enemy_stableobstacle_2))
  (bind _staticmesh_enemy_2 (Variables|/Game/Core/Terrain/Enemy/BP_Enemy.BP_Enemy_C|GetStaticMesh_Enemy _enemy_stableobstacle))
  (Variables|Default|SetIsSpawnObstacle false)
  (Rendering|SetVisibility _staticmesh_enemy_2 false false)
  (Development|SetHiddeninGame _staticmesh_enemy_2 true false)
  (Collision|SetCollisionEnabled _staticmesh_enemy "NoCollision")
  (Collision|SetCollisionResponsetoAllChannels _staticmesh_enemy "ECR_Ignore"))

(fn ShowCollectableBulletonGrid
  (bind _collectableitem_bullet (Variables|Default|GetCollectableItem_Bullet))
  (bind _collectableitem_bullet_2 (Variables|Default|GetCollectableItem_Bullet))
  (bind _collectableitem_bullet_3 (Variables|Default|GetCollectableItem_Bullet))
  (bind _staticmesh_collectableitem (Variables|/Game/Core/Terrain/CollectableItem/BP_CollectableItem.BP_CollectableItem_C|GetStaticMesh_CollectableItem _collectableitem_bullet))
  (bind _sphere_collectableitem_collision (Variables|/Game/Core/Terrain/CollectableItem/BP_CollectableItem.BP_CollectableItem_C|GetSphere_CollectableItem_Collision _collectableitem_bullet_3))
  (Variables|Default|SetIsSpawnCollectableBullet true)
  (Rendering|SetVisibility _staticmesh_collectableitem true false)
  (Development|SetHiddeninGame _staticmesh_collectableitem false false)
  (Collision|SetCollisionEnabled _sphere_collectableitem_collision "QueryOnly")
  (Collision|SetCollisionResponsetoChannel _sphere_collectableitem_collision "ECC_Pawn" "ECR_Overlap")
  (Default|UpdateDynamicMaterialandColor _collectableitem_bullet_2)
  (Variables|Default|SetItemColor (Variables|/Game/Core/Terrain/CollectableItem/BP_CollectableItem.BP_CollectableItem_C|GetCurrentColor _collectableitem_bullet_2)))

(fn DestroyCollectableBulletonGrid
  (bind _collectableitem_bullet (Variables|Default|GetCollectableItem_Bullet))
  (bind _collectableitem_bullet_2 (Variables|Default|GetCollectableItem_Bullet))
  (bind _staticmesh_collectableitem (Variables|/Game/Core/Terrain/CollectableItem/BP_CollectableItem.BP_CollectableItem_C|GetStaticMesh_CollectableItem _collectableitem_bullet))
  (bind _sphere_collectableitem_collision (Variables|/Game/Core/Terrain/CollectableItem/BP_CollectableItem.BP_CollectableItem_C|GetSphere_CollectableItem_Collision _collectableitem_bullet_2))
  (Variables|Default|SetIsSpawnCollectableBullet false)
  (Rendering|SetVisibility _staticmesh_collectableitem false false)
  (Development|SetHiddeninGame _staticmesh_collectableitem true false)
  (Collision|SetCollisionEnabled _sphere_collectableitem_collision "NoCollision")
  (Collision|SetCollisionResponsetoAllChannels _sphere_collectableitem_collision "ECR_Ignore"))

(fn ShowIncreaseSpeedonGrid
  (bind _collectableitem_speedincrease (Variables|Default|GetCollectableItem_SpeedIncrease))
  (bind _collectableitem_speedincrease_2 (Variables|Default|GetCollectableItem_SpeedIncrease))
  (bind _staticmesh_collectableitem (Variables|/Game/Core/Terrain/CollectableItem/BP_CollectableItem.BP_CollectableItem_C|GetStaticMesh_CollectableItem _collectableitem_speedincrease_2))
  (bind _sphere_collectableitem_collision (Variables|/Game/Core/Terrain/CollectableItem/BP_CollectableItem.BP_CollectableItem_C|GetSphere_CollectableItem_Collision _collectableitem_speedincrease))
  (Variables|Default|SetIsSpawnIncreaseSpeedOnGrid true)
  (Rendering|SetVisibility _staticmesh_collectableitem true false)
  (Development|SetHiddeninGame _staticmesh_collectableitem false false)
  (Collision|SetCollisionEnabled _sphere_collectableitem_collision "QueryOnly")
  (Collision|SetCollisionResponsetoChannel _sphere_collectableitem_collision "ECC_Pawn" "ECR_Overlap"))

(fn DestroyIncreaseSpeedonGrid
  (bind _collectableitem_speedincrease (Variables|Default|GetCollectableItem_SpeedIncrease))
  (bind _collectableitem_speedincrease_2 (Variables|Default|GetCollectableItem_SpeedIncrease))
  (bind _staticmesh_collectableitem (Variables|/Game/Core/Terrain/CollectableItem/BP_CollectableItem.BP_CollectableItem_C|GetStaticMesh_CollectableItem _collectableitem_speedincrease_2))
  (bind _sphere_collectableitem_collision (Variables|/Game/Core/Terrain/CollectableItem/BP_CollectableItem.BP_CollectableItem_C|GetSphere_CollectableItem_Collision _collectableitem_speedincrease))
  (Variables|Default|SetIsSpawnIncreaseSpeedOnGrid false)
  (Rendering|SetVisibility _staticmesh_collectableitem false false)
  (Development|SetHiddeninGame _staticmesh_collectableitem true false)
  (Collision|SetCollisionEnabled _sphere_collectableitem_collision "NoCollision")
  (Collision|SetCollisionResponsetoAllChannels _sphere_collectableitem_collision "ECR_Ignore"))

(fn ShowCoinonGrid
  (bind _collectableitem_coin (Variables|Default|GetCollectableItem_Coin))
  (bind _collectableitem_coin_2 (Variables|Default|GetCollectableItem_Coin))
  (bind _collectableitem_coin_3 (Variables|Default|GetCollectableItem_Coin))
  (bind _staticmesh_collectableitem (Variables|/Game/Core/Terrain/CollectableItem/BP_CollectableItem.BP_CollectableItem_C|GetStaticMesh_CollectableItem _collectableitem_coin_2))
  (bind _sphere_collectableitem_collision (Variables|/Game/Core/Terrain/CollectableItem/BP_CollectableItem.BP_CollectableItem_C|GetSphere_CollectableItem_Collision _collectableitem_coin_3))
  (Variables|Default|SetIsSpawnCollectableCoin true)
  (Rendering|SetVisibility _staticmesh_collectableitem true false)
  (Development|SetHiddeninGame _staticmesh_collectableitem false false)
  (Collision|SetCollisionEnabled _sphere_collectableitem_collision "QueryOnly")
  (Collision|SetCollisionResponsetoChannel _sphere_collectableitem_collision "ECC_Pawn" "ECR_Overlap")
  (Default|UpdateDynamicMaterialandColor _collectableitem_coin)
  (Variables|Default|SetItemColor (Variables|/Game/Core/Terrain/CollectableItem/BP_CollectableItem.BP_CollectableItem_C|GetCurrentColor _collectableitem_coin))
  (Default|StartRotateCoinforLoop _collectableitem_coin))

(fn DestroyCoinonGrid
  (bind _collectableitem_coin (Variables|Default|GetCollectableItem_Coin))
  (bind _collectableitem_coin_2 (Variables|Default|GetCollectableItem_Coin))
  (bind _staticmesh_collectableitem (Variables|/Game/Core/Terrain/CollectableItem/BP_CollectableItem.BP_CollectableItem_C|GetStaticMesh_CollectableItem _collectableitem_coin_2))
  (bind _sphere_collectableitem_collision (Variables|/Game/Core/Terrain/CollectableItem/BP_CollectableItem.BP_CollectableItem_C|GetSphere_CollectableItem_Collision _collectableitem_coin))
  (Variables|Default|SetIsSpawnCollectableCoin false)
  (Rendering|SetVisibility _staticmesh_collectableitem false false)
  (Development|SetHiddeninGame _staticmesh_collectableitem true false)
  (Collision|SetCollisionEnabled _sphere_collectableitem_collision "NoCollision")
  (Collision|SetCollisionResponsetoAllChannels _sphere_collectableitem_collision "ECR_Ignore")
  (Default|StopCoinforLoop (Variables|Default|GetCollectableItem_Coin)))

(fn ShowMoveEnemyonGrid
  (bind _enemy_moveableenemy (Variables|Default|GetEnemy_MoveableEnemy))
  (bind _enemy_moveableenemy_2 (Variables|Default|GetEnemy_MoveableEnemy))
  (bind _enemy_moveableenemy_3 (Variables|Default|GetEnemy_MoveableEnemy))
  (bind _staticmesh_enemy (Variables|/Game/Core/Terrain/Enemy/BP_Enemy.BP_Enemy_C|GetStaticMesh_Enemy _enemy_moveableenemy))
  (bind _staticmesh_enemy_2 (Variables|/Game/Core/Terrain/Enemy/BP_Enemy.BP_Enemy_C|GetStaticMesh_Enemy _enemy_moveableenemy_2))
  (Variables|Default|SetIsSpawnMoveEnemy true)
  (Rendering|SetVisibility _staticmesh_enemy true false)
  (Development|SetHiddeninGame _staticmesh_enemy false false)
  (Collision|SetCollisionEnabled _staticmesh_enemy_2 "QueryOnly")
  (Collision|SetCollisionResponsetoChannel _staticmesh_enemy_2 "ECC_Pawn" "ECR_Overlap")
  (Collision|SetCollisionResponsetoChannel _staticmesh_enemy_2 "ECC_GameTraceChannel2" "ECR_Overlap")
  (Collision|SetCollisionResponsetoChannel _staticmesh_enemy_2 "ECC_GameTraceChannel6" "ECR_Block")
  (Default|UpdateEnemyDynamicMaterialandColor _enemy_moveableenemy_3)
  (Variables|Default|SetItemColor (Variables|/Game/Core/Terrain/Enemy/BP_Enemy.BP_Enemy_C|GetCurrentColor _enemy_moveableenemy_3))
  (Default|StartMoveEnemyRelativeLocationforLoop (Variables|Default|GetEnemy_MoveableEnemy)))

(fn DestroyMoveEnemyonGrid
  (bind _enemy_moveableenemy (Variables|Default|GetEnemy_MoveableEnemy))
  (bind _enemy_moveableenemy_2 (Variables|Default|GetEnemy_MoveableEnemy))
  (bind _staticmesh_enemy (Variables|/Game/Core/Terrain/Enemy/BP_Enemy.BP_Enemy_C|GetStaticMesh_Enemy _enemy_moveableenemy_2))
  (bind _staticmesh_enemy_2 (Variables|/Game/Core/Terrain/Enemy/BP_Enemy.BP_Enemy_C|GetStaticMesh_Enemy _enemy_moveableenemy))
  (Variables|Default|SetIsSpawnMoveEnemy false)
  (Rendering|SetVisibility _staticmesh_enemy_2 false false)
  (Development|SetHiddeninGame _staticmesh_enemy_2 true false)
  (Collision|SetCollisionEnabled _staticmesh_enemy "NoCollision")
  (Collision|SetCollisionResponsetoAllChannels _staticmesh_enemy "ECR_Ignore")
  (Default|StopEnemyRelationLocationMovementandResetState (Variables|Default|GetEnemy_MoveableEnemy)))

(fn ShowShotableEnemyonGrid
  (bind _enemy_shotableenemy (Variables|Default|GetEnemy_ShotableEnemy))
  (bind _enemy_shotableenemy_2 (Variables|Default|GetEnemy_ShotableEnemy))
  (bind _enemy_shotableenemy_3 (Variables|Default|GetEnemy_ShotableEnemy))
  (bind _staticmesh_enemy (Variables|/Game/Core/Terrain/Enemy/BP_Enemy.BP_Enemy_C|GetStaticMesh_Enemy _enemy_shotableenemy))
  (bind _staticmesh_enemy_2 (Variables|/Game/Core/Terrain/Enemy/BP_Enemy.BP_Enemy_C|GetStaticMesh_Enemy _enemy_shotableenemy_3))
  (Variables|Default|SetIsSpawnShotableEnemy true)
  (Rendering|SetVisibility _staticmesh_enemy true false)
  (Development|SetHiddeninGame _staticmesh_enemy false false)
  (Collision|SetCollisionEnabled _staticmesh_enemy_2 "QueryOnly")
  (Collision|SetCollisionResponsetoChannel _staticmesh_enemy_2 "ECC_Pawn" "ECR_Overlap")
  (Collision|SetCollisionResponsetoChannel _staticmesh_enemy_2 "ECC_GameTraceChannel2" "ECR_Overlap")
  (Collision|SetCollisionResponsetoChannel _staticmesh_enemy_2 "ECC_GameTraceChannel6" "ECR_Block")
  (Default|UpdateEnemyDynamicMaterialandColor _enemy_shotableenemy_2)
  (Variables|Default|SetItemColor (Variables|/Game/Core/Terrain/Enemy/BP_Enemy.BP_Enemy_C|GetCurrentColor _enemy_shotableenemy_2))
  (Default|StartDetectPlayer (Variables|Default|GetEnemy_ShotableEnemy)))

(fn DestroyShotableEnemyonGrid
  (bind _enemy_shotableenemy (Variables|Default|GetEnemy_ShotableEnemy))
  (bind _enemy_shotableenemy_2 (Variables|Default|GetEnemy_ShotableEnemy))
  (bind _staticmesh_enemy (Variables|/Game/Core/Terrain/Enemy/BP_Enemy.BP_Enemy_C|GetStaticMesh_Enemy _enemy_shotableenemy_2))
  (bind _staticmesh_enemy_2 (Variables|/Game/Core/Terrain/Enemy/BP_Enemy.BP_Enemy_C|GetStaticMesh_Enemy _enemy_shotableenemy))
  (Variables|Default|SetIsSpawnShotableEnemy false)
  (Rendering|SetVisibility _staticmesh_enemy_2 false false)
  (Development|SetHiddeninGame _staticmesh_enemy_2 true false)
  (Collision|SetCollisionEnabled _staticmesh_enemy "NoCollision")
  (Collision|SetCollisionResponsetoAllChannels _staticmesh_enemy "ECR_Ignore")
  (Default|StopDetectPlayerAircraftandReset (Variables|Default|GetEnemy_ShotableEnemy)))