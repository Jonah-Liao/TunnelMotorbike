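; BP_CombatSystem runs a round of the running combat game, from start and pause to end, tracking score and distance.
; On BeginPlay it creates the combat screen, terrain and player pawn, passing itself to each.
; Pawn weapon and input-device events refresh on-screen control tips.
; Ending a round inserts the result into a sorted top-15 leaderboard, saved as JSON through the game instance, and names can be linked to records afterwards.
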(event EventBeginPlay
  (SaveAndLoad|GetGameInstanceandLoadJsonDataandSavedGameData)
  (bind _outvalue (|GetJsonField (Variables|SaveAndLoad|GetCurrentJsonData) "HighScore Board Info"))
  (Variables|SaveAndLoad|SetHighscoreRecord _outvalue)
  ;[0 0 0 0.5] Create Combat Widget UI
  (bind _returnvalue (UserInterface|CreateWidget "/Game/Core/MenuUi/CombatScreen/WBP_CombatScreen.WBP_CombatScreen_C" 0 self))
  (bind _output_get (Variables|Default|SetCreatedCombatScreen _returnvalue))
  (UserInterface|Viewport|AddtoViewport _output_get 0)
  (Default|SwitchBigButtonAppearance (Variables|Default|GetCreatedCombatScreen) "NewEnumerator0")
  (EventDispatchers|BindEventtoOnPlayerClickedPlayAgaininCombatMenu (Variables|Default|GetCreatedCombatScreen) (EventDispatchers|CreateEvent :!event OnPlayerClickedPlayAgaininCombatMenu))
  (Default|UpdateKeyImageIconandText (Variables|/Game/Core/MenuUi/CombatScreen/WBP_CombatScreen.WBP_CombatScreen_C|GetWBP_ControlTips (Variables|Default|GetCreatedCombatScreen)) (KeyTips|GetKeyNameDataArrayfromKeyTypes (Variables|ControlTips|GetKeyTipsBeforeStartGame)) "NewEnumerator0")
  (Default|UpdateControlTipsSize (Variables|/Game/Core/MenuUi/CombatScreen/WBP_CombatScreen.WBP_CombatScreen_C|GetWBP_ControlTips (Variables|Default|GetCreatedCombatScreen)) (Variables|ControlTips|GetControlTipsSizeBeforeStartGame))
  ;[0 0 0 0.5] Comment
  (bind _output_get_2 (Variables|Default|SetTransfomOfTerrainGridWithPlayer (Math|Transform|MakeTransform "0, 0, 0")))
  (bind _returnvalue_2 (Game|SpawnActorfromClass "/Game/Core/Terrain/BP_Terrain.BP_Terrain_C" _output_get_2 "Undefined" "MultiplyWithRoot" 0 self 0))
  (Variables|Default|SetTerrain _returnvalue_2)
  ;[0 0 0 0.5] Spawn BP_Pawn , Input basic data
  (bind _returnvalue_3 (Game|SpawnActorfromClass "/Game/Core/Utilities/BP_Pawn.BP_Pawn_C" (Math|Transform|MakeTransform (Math|Vector|MakeVector (.X (Math|Vector|BreakVector (.Location (Math|Transform|BreakTransform (Variables|Default|GetTransfomOfTerrainGridWithPlayer))))) (.Y (Math|Vector|BreakVector (.Location (Math|Transform|BreakTransform (Variables|Default|GetTransfomOfTerrainGridWithPlayer))))) (+ (.Z (Math|Vector|BreakVector (.Location (Math|Transform|BreakTransform (Variables|Default|GetTransfomOfTerrainGridWithPlayer))))) (Variables|Default|GetHeightBetweenPlayerAndGrid) (* (Default|GetDistanceBetweenCenterandGridCenter (Variables|Default|GetTerrain)) -1.0))) (.Rotation (Math|Transform|BreakTransform (Variables|Default|GetTransfomOfTerrainGridWithPlayer))) (.Scale (Math|Transform|BreakTransform (Variables|Default|GetTransfomOfTerrainGridWithPlayer)))) "Undefined" "MultiplyWithRoot" 0 self 0))
  (bind _output_get_3 (Variables|Default|SetPlayerPawn _returnvalue_3))
  (EventDispatchers|BindEventtoOnPlayerEquippedWeapon _output_get_3 (EventDispatchers|CreateEvent :!event OnPlayerEquippedWeapon))
  (EventDispatchers|BindEventtoOnPlayerWeaponExpired _output_get_3 (EventDispatchers|CreateEvent :!event OnPlayerWeaponExpiredorWithoutItem))
  (EventDispatchers|BindEventtoOnPlayerInputDeviceTypeChanged _output_get_3 (EventDispatchers|CreateEvent :!event OnPlayerInputDeviceTypeChanged))
  (Variables|/Game/Core/Utilities/BP_Pawn.BP_Pawn_C|SetIsEnableCombatInput _output_get_3 true)
  (Pawn|Possess (Game|GetPlayerController 0) (Variables|Default|GetPlayerPawn)))

(fn ConstructionScript)

(fn SetIsPauseGameDurringCombat
  (params (IsPauseGame :type Boolean))
  (bind _output_get (Variables|Default|SetIsGamePausedDuringCombat IsPauseGame))
  (if _output_get
    (Default|StopTunnelMovement (Variables|Default|GetTerrain))
    (Default|CallOnCombatPaused)
    (Variables|/Script/Engine.PlayerController|SetbShowMouseCursor (Game|GetPlayerController 0) (Variables|Default|GetIsGamePausedDuringCombat))
    (Default|IsShowCombatOption (Variables|Default|GetCreatedCombatScreen) true)
    (else
      (Default|StartTimerOfTerrianMovement (Variables|Default|GetTerrain))
      (Default|CallOnCombatContinue)
      (Variables|/Script/Engine.PlayerController|SetbShowMouseCursor (Game|GetPlayerController 0) (Variables|Default|GetIsGamePausedDuringCombat))
      (Default|IsShowCombatOption (Variables|Default|GetCreatedCombatScreen) false))))

(fn StartCombat
  (bind _createdcombatscreen (Variables|Default|GetCreatedCombatScreen))
  (bind _createdcombatscreen_2 (Variables|Default|GetCreatedCombatScreen))
  ;[0.15 0.15 0.15 0.5] Comment
  (if (not (Variables|Default|GetIsStartCombat))
    (Variables|Default|SetIsStartCombat true)
    (Variables|Default|SetIsGamePausedDuringCombat false)
    (Variables|/Script/Engine.PlayerController|SetbShowMouseCursor (Game|GetPlayerController 0) false)
    ;[0.15 0.15 0.15 0.5] Comment
    (Default|SetAimLockerandRelatedUiElementVisibility _createdcombatscreen_2 false)
    (Default|SwitchBigButtonAppearance _createdcombatscreen_2 "NewEnumerator1")
    (KeyTips|OnPlayerWeaponExpiredorWithoutItem)
    (bind _output_get (Variables|SaveAndLoad|SetCurrentScore 0))
    (Default|SetRecordedScore _createdcombatscreen _output_get)
    (bind _output_get_2 (Variables|SaveAndLoad|SetCurrentDistance 0))
    (Default|SetRecordedPassDistance _createdcombatscreen _output_get_2)
    (Default|CallOnCombatStart)))

(fn EndCombat
  (bind _createdcombatscreen (Variables|Default|GetCreatedCombatScreen))
  (bind _createdcombatscreen_2 (Variables|Default|GetCreatedCombatScreen))
  (if (Variables|Default|GetIsStartCombat)
    (Variables|Default|SetIsStartCombat false))
  (Variables|Default|SetIsGamePausedDuringCombat false)
  (Default|CallOnCombatEnd)
  ;[0.15 0.15 0.15 0.5] Comment
  (Default|SetAimLockerandRelatedUiElementVisibility _createdcombatscreen_2 false)
  (Default|IsShowCombatOption _createdcombatscreen_2 false)
  (Variables|/Script/Engine.PlayerController|SetbShowMouseCursor (Game|GetPlayerController 0) true)
  ;[0.15 0.15 0.15 0.5] Comment
  (Utilities|Array|Add (Variables|SaveAndLoad|GetHighscoreRecord) (Utilities|Struct|MakeS_HighscoreUnitDetail (Variables|SaveAndLoad|GetCurrentPlayerName) (Variables|SaveAndLoad|GetCurrentScore) (Variables|SaveAndLoad|GetCurrentDistance)))
  ;[0.15 0.15 0.15 0.5] Comment
  (bind _output_get (Variables|SaveAndLoad|SetHighscoreRecord (SaveAndLoad|ReorderHighscoreArray (Variables|SaveAndLoad|GetHighscoreRecord) true 15)))
  (|SetJsonField (Variables|SaveAndLoad|GetCurrentJsonData) "HighScore Board Info" _output_get)
  (SaveAndLoad|SaveNewDatatoGameInstance (Variables|SaveAndLoad|GetCurrentGameData) (Variables|SaveAndLoad|GetCurrentJsonData))
  ;[0.15 0.15 0.15 0.5] Comment
  (Default|IsShowCombatEndMenu _createdcombatscreen true)
  (Default|IsShowCombatControlButton _createdcombatscreen false))

(fn ReorderHighscoreArray
  (params (OriginalArray :type Array%20of%20S%20Highscore%20Unit%20Detail%20Structures) (IsBigToSmall :type Boolean) (DataNumToContain :type Integer))
  (for _array_element OriginalArray
    (LocalVariables|SetCurrentAddData _array_element)
    (if (> (Utilities|Array|Length (LocalVariables|GetReArrayHighscoreData)) 0)
      (LocalVariables|SetIsCurrentDataTheSmallestOrBiggestOne true)
      (bind (_array_element_2 _array_index) (Utilities|Array|ForEachLoopwithBreak (LocalVariables|GetReArrayHighscoreData) :!label _label)
        (:LoopBody
          (LocalVariables|SetCompareData _array_element_2)
          (if IsBigToSmall
            (if (not (< (Utilities|Struct|BreakS_HighscoreUnitDetail (LocalVariables|GetCurrentAddData)) (Utilities|Struct|BreakS_HighscoreUnitDetail (LocalVariables|GetCompareData))))
              (LocalVariables|SetIsCurrentDataTheSmallestOrBiggestOne false :!label _label_2)
              (Utilities|Array|Insert (LocalVariables|GetReArrayHighscoreData) (LocalVariables|GetCurrentAddData) _array_index)
              (goto _label Break))
            (elif (not (> (Utilities|Struct|BreakS_HighscoreUnitDetail (LocalVariables|GetCurrentAddData)) (Utilities|Struct|BreakS_HighscoreUnitDetail (LocalVariables|GetCompareData))))
              (goto _label_2))))
        (:Completed
          (if (LocalVariables|GetIsCurrentDataTheSmallestOrBiggestOne)
            (Utilities|Array|Add (LocalVariables|GetReArrayHighscoreData) (LocalVariables|GetCurrentAddData)))))
      (else
        (Utilities|Array|Add (LocalVariables|GetReArrayHighscoreData) (LocalVariables|GetCurrentAddData)))))
  (bind (_array_element_3 _array_index_2) (Utilities|Array|ForEachLoopwithBreak (LocalVariables|GetReArrayHighscoreData) :!label _label_3)
    (:LoopBody
      (if (<= _array_index_2 (- DataNumToContain 1))
        (Utilities|Array|Add (LocalVariables|GetRetArray) _array_element_3)
        (else
          (goto _label_3 Break))))
    (:Completed
      (return (LocalVariables|GetRetArray)))))

(fn GetGameInstanceandLoadJsonDataandSavedGameData
  (bind _output_get (Variables|SaveAndLoad|SetCurrentGameInstance (.AsBP%20Game%20Instance (Utilities|Casting|CastToBP_GameInstance (Game|GetGameInstance)))))
  (Variables|SaveAndLoad|SetCurrentJsonData (Variables|/Game/Core/SaveGame/BP_GameInstance.BP_GameInstance_C|GetSavedJsonData _output_get))
  (Variables|SaveAndLoad|SetCurrentGameData (Variables|/Game/Core/SaveGame/BP_GameInstance.BP_GameInstance_C|GetSavedData _output_get)))

(fn LinkPlayerNametoSpecificScoreRecord
  (params (NewPlayerName :type Text) (Score :type Integer) (Distance :type Integer))
  (LocalVariables|SetIsFindTargetPlayer false)
  (bind _output_get (LocalVariables|SetOldHighScoreRecord (Variables|SaveAndLoad|GetHighscoreRecord)))
  (bind (_array_element _array_index) (Utilities|Array|ForEachLoopwithBreak _output_get :!label _label)
    (:LoopBody
      (LocalVariables|SetIndex _array_index)
      (bind _output_get_2 (LocalVariables|SetHighscoreDetail _array_element))
      (if (and (== (.Score (Utilities|Struct|BreakS_HighscoreUnitDetail _output_get_2)) Score) (== (.Distance (Utilities|Struct|BreakS_HighscoreUnitDetail _output_get_2)) Distance))
        (LocalVariables|SetIsFindTargetPlayer true)
        (bind _output_get_3 (Variables|SaveAndLoad|SetCurrentPlayerName (Utilities|String|ToString(Text) NewPlayerName)))
        (Utilities|Array|SetArrayElem (Variables|SaveAndLoad|GetHighscoreRecord) (LocalVariables|GetIndex) (Utilities|Struct|MakeS_HighscoreUnitDetail _output_get_3 Score Distance))
        (goto _label Break)))
    (:Completed
      (if (LocalVariables|GetIsFindTargetPlayer)
        (bind _output_get_4 (Variables|SaveAndLoad|SetHighscoreRecord (SaveAndLoad|ReorderHighscoreArray (Variables|SaveAndLoad|GetHighscoreRecord) true 15)))
        (|SetJsonField (Variables|SaveAndLoad|GetCurrentJsonData) "HighScore Board Info" _output_get_4)
        (Default|UpdateHighscoreDataBaseonPlatform (Variables|Default|GetCreatedCombatScreen) (Variables|SaveAndLoad|GetHighscoreRecord))
        (SaveAndLoad|SaveNewDatatoGameInstance (Variables|SaveAndLoad|GetCurrentGameData) (Variables|SaveAndLoad|GetCurrentJsonData))))))

(fn SaveNewDatatoGameInstance
  (params (NewGameData :type BP%20Save%20Game%20Object%20Reference) (NewJsonData :type Json%20Object%20Wrapper%20Structure))
  (bind _returnvalue (Game|GetGameInstance))
  (bind _asbp_game_instance (Utilities|Casting|CastToBP_GameInstance _returnvalue))
  (Variables|/Game/Core/SaveGame/BP_GameInstance.BP_GameInstance_C|SetSavedData _asbp_game_instance NewGameData)
  (Variables|/Game/Core/SaveGame/BP_GameInstance.BP_GameInstance_C|SetSavedJsonData _asbp_game_instance NewJsonData)
  (Default|SaveGameData _asbp_game_instance false))

(fn AddScore
  (params (DetlaScore :type Integer))
  (bind _createdcombatscreen (Variables|Default|GetCreatedCombatScreen))
  (Variables|SaveAndLoad|SetCurrentScore (+ DetlaScore (Variables|SaveAndLoad|GetCurrentScore)))
  (Utilities|IsValid _createdcombatscreen
    (:Is%20Valid
      (Default|SetRecordedScore _createdcombatscreen (Variables|SaveAndLoad|GetCurrentScore)))))

(fn GetKeyNameDataArrayfromKeyTypes
  (params (KeyNameArray :type Array%20of%20E_KeyName%20Enums :default "NewEnumerator0"))
  (for _array_element KeyNameArray
    (Utilities|Array|Add (LocalVariables|GetRetKeyDataArray) (CallFunction|GetKeyDatafromKeyType _array_element)))
  (return (LocalVariables|GetRetKeyDataArray)))

(fn OnPlayerEquippedWeapon
  (bind _createdcombatscreen (Variables|Default|GetCreatedCombatScreen))
  (bind _wbp_controltips (Variables|/Game/Core/MenuUi/CombatScreen/WBP_CombatScreen.WBP_CombatScreen_C|GetWBP_ControlTips _createdcombatscreen))
  ;[0.15 0.15 0.15 0.5] Comment
  (Default|UpdateKeyImageIconandText _wbp_controltips (KeyTips|GetKeyNameDataArrayfromKeyTypes (Variables|ControlTips|GetKeyTipsWhenEquippedWeapon)) (Variables|/Game/Core/Utilities/BP_Pawn.BP_Pawn_C|GetCurrentInputDeviceType (Variables|Default|GetPlayerPawn)))
  (Default|UpdateControlTipsSize _wbp_controltips (Variables|ControlTips|GetControlTipsSizeWhenEquippedWeapon)))

(fn OnPlayerWeaponExpiredorWithoutItem
  (bind _createdcombatscreen (Variables|Default|GetCreatedCombatScreen))
  (bind _wbp_controltips (Variables|/Game/Core/MenuUi/CombatScreen/WBP_CombatScreen.WBP_CombatScreen_C|GetWBP_ControlTips _createdcombatscreen))
  ;[0.15 0.15 0.15 0.5] Comment
  (Default|UpdateKeyImageIconandText _wbp_controltips (KeyTips|GetKeyNameDataArrayfromKeyTypes (Variables|ControlTips|GetKeyTipsWhenRunningWithoutItem)) (Variables|/Game/Core/Utilities/BP_Pawn.BP_Pawn_C|GetCurrentInputDeviceType (Variables|Default|GetPlayerPawn)))
  (Default|UpdateControlTipsSize _wbp_controltips (Variables|ControlTips|GetControlTipsSizeWhenRunWithoutItem)))

(fn OnPlayerClickedPlayAgaininCombatMenu
  (Game|OpenLevel(byObjectReference) "/Game/Map/L_RunningMap.L_RunningMap"))

(fn OnPlayerInputDeviceTypeChanged
  (params (NewDeviceInputType :type E_InputDeviceType%20Enum :default "NewEnumerator0"))
  (bind _createdcombatscreen (Variables|Default|GetCreatedCombatScreen))
  (bind _wbp_controltips (Variables|/Game/Core/MenuUi/CombatScreen/WBP_CombatScreen.WBP_CombatScreen_C|GetWBP_ControlTips _createdcombatscreen))
  (bind _output_get (LocalVariables|SetNewLocalVar (Variables|/Game/Core/MenuUi/CombatScreen/WBP_ControlTips.WBP_ControlTips_C|GetCurrentKeyIconAndTextArray _wbp_controltips)))
  (Default|UpdateKeyImageIconandText _wbp_controltips _output_get NewDeviceInputType)
  (Default|UpdateControlTipsSize _wbp_controltips (Variables|/Game/Core/MenuUi/CombatScreen/WBP_ControlTips.WBP_ControlTips_C|GetCurrentControlTipsSize _wbp_controltips)))