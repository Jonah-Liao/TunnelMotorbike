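; BP_PlayerBullet is the player's projectile, spawning hidden with collision off and tinted by a dynamic material.
; ShootOutBullet enables collision, places it at the pawn's bullet child actor with random X jitter, and starts a looping timer.
; The timer, rather than Tick, steps it along +X until it passes the track's end.
; Overlaps destroy obstacles or enemies on terrain units along with the bullet; enemy bullets also destroy it.
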(event OnComponentBeginOverlap(BulletCollision)
  (params (OverlappedComponent :type Primitive%20Component%20Object%20Reference) (OtherActor :type Actor%20Object%20Reference) (OtherComp :type Primitive%20Component%20Object%20Reference) (OtherBodyIndex :type Integer) (bFromSweep :type Boolean) (SweepResult :type Hit%20Result%20Structure%20%28by%20ref%29))
  ;[0.15 0.15 0.15 0.5] Comment
  (Utilities|IsValid OtherActor
    (:Is%20Valid
      (bind _asbp_terrain_unit (Utilities|Casting|CastToBP_TerrainUnit (Actor|GetAttachParentActor OtherActor))
        (:then
          (CallFunction|CompletedBulletShoot)
          (Variables|Default|SetHitGridWithCube _asbp_terrain_unit)
          (if (Variables|/Game/Core/Terrain/BP_TerrainUnit.BP_TerrainUnit_C|GetIsSpawnObstacle (Variables|Default|GetHitGridWithCube))
            (Default|DestroyObstacleonGrid (Variables|Default|GetHitGridWithCube))
            (Actor|DestroyActor :!label _label)
            (elif (Variables|/Game/Core/Terrain/BP_TerrainUnit.BP_TerrainUnit_C|GetIsSpawnMoveEnemy (Variables|Default|GetHitGridWithCube))
              (Default|DestroyMoveEnemyonGrid (Variables|Default|GetHitGridWithCube))
              (goto _label)
              (elif (Variables|/Game/Core/Terrain/BP_TerrainUnit.BP_TerrainUnit_C|GetIsSpawnShotableEnemy (Variables|Default|GetHitGridWithCube))
                (Default|DestroyShotableEnemyonGrid (Variables|Default|GetHitGridWithCube))
                (goto _label)))))
        (:CastFailed
          (Utilities|Casting|CastToBP_EnemyShotBullet OtherActor)
          (Actor|DestroyActor))))))

(event Custom|ShootOutBullet
  (bind _playerpawn (Variables|Default|GetPlayerPawn))
  (bind _bulletcollision (Variables|Default|GetBulletCollision))
  (bind _childactor_bullet (Variables|/Game/Core/Utilities/BP_Pawn.BP_Pawn_C|GetChildActor_Bullet _playerpawn))
  (bind _returnvalue (Transformation|GetWorldTransform _childactor_bullet))
  (bind (_location _rotation _scale) (Math|Transform|BreakTransform _returnvalue))
  (bind (_x _y _z) (Math|Vector|BreakVector _location))
  ;[0.15 0.15 0.15 0.5] Comment
  (Utilities|IsValid _bulletcollision
    (:Is%20Valid
      (Collision|SetCollisionEnabled _bulletcollision "QueryOnly")
      (Collision|SetCollisionResponsetoChannel _bulletcollision "ECC_GameTraceChannel1" "ECR_Overlap")
      (Collision|SetCollisionResponsetoChannel _bulletcollision "ECC_GameTraceChannel5" "ECR_Block")
      (bind _output_get (Variables|Default|SetShootOutStartTransform (Math|Transform|MakeTransform (Math|Vector|MakeVector (+ _x (Math|Random|RandomFloatinRange -15.0 1e+01)) _y _z) _rotation _scale)))
      (Transformation|SetActorTransform _output_get)
      (Variables|Default|SetCurrentTransform (Variables|Default|GetShootOutStartTransform))
      (CallFunction|StarttoMoveBullet))))

(event Custom|StartToMoveBullet
  ;[0.15 0.15 0.15 0.5] Comment
  (bind _returnvalue (Utilities|Time|SetTimerbyEvent (delegate Custom|MovingBullet) 0.04 true))
  (Variables|Default|SetBulletMoveTimer _returnvalue))

(event Custom|CompletedBulletShoot
  ;[0.15 0.15 0.15 0.5] Comment
  (Utilities|Time|ClearandInvalidateTimerbyHandle (Variables|Default|GetBulletMoveTimer)))

(event Custom|MovingBullet
  (bind _combatsystem (Variables|Default|GetCombatSystem))
  (bind _terrain (Variables|/Game/Core/CombatSystem/BP_CombatSystem.BP_CombatSystem_C|GetTerrain _combatsystem))
  ;[0.15 0.15 0.15 0.5] Comment
  (Rendering|SetActorHiddenInGame false)
  ;[0.15 0.15 0.15 0.5] Comment
  (CallFunction|MoveBulletForeward)
  (if (> (.X (Math|Vector|BreakVector (.Location (Math|Transform|BreakTransform (Variables|Default|GetCurrentTransform))))) (* (Variables|/Game/Core/Terrain/BP_Terrain.BP_Terrain_C|GetGridNumberInATrack _terrain) (.X (Math|Vector2D|BreakVector2D (Variables|/Game/Core/Terrain/BP_Terrain.BP_Terrain_C|GetGridSize _terrain)))))
    (CallFunction|CompletedBulletShoot)
    (Actor|DestroyActor)))

(event EventTick
  (params (DeltaSeconds :type Float%20%28single-precision%29)))

(event EventBeginPlay
  (bind _bulletcollision (Variables|Default|GetBulletCollision))
  ;[0.15 0.15 0.15 0.5] Comment
  (Rendering|SetActorHiddenInGame true)
  (CallFunction|SetBulletColorMaterial)
  (Collision|SetCollisionEnabled _bulletcollision "NoCollision")
  (Collision|SetCollisionResponsetoChannel _bulletcollision "ECC_GameTraceChannel1" "ECR_Ignore"))

(fn ConstructionScript)

(fn MoveBulletForeward
  ;[0.15 0.15 0.15 0.5] Comment
  (Transformation|SetActorTransform (Math|Transform|MakeTransform (Math|Vector|MakeVector (+ (.X (Math|Vector|BreakVector (.Location (Math|Transform|BreakTransform (Variables|Default|GetCurrentTransform))))) (Variables|Default|GetBulletSpeed)) (.Y (Math|Vector|BreakVector (.Location (Math|Transform|BreakTransform (Variables|Default|GetCurrentTransform))))) (.Z (Math|Vector|BreakVector (.Location (Math|Transform|BreakTransform (Variables|Default|GetCurrentTransform)))))) (.Rotation (Math|Transform|BreakTransform (Variables|Default|GetCurrentTransform))) (.Scale (Math|Transform|BreakTransform (Variables|Default|GetCurrentTransform)))))
  (Variables|Default|SetCurrentTransform (Math|Transform|MakeTransform (Math|Vector|MakeVector (+ (.X (Math|Vector|BreakVector (.Location (Math|Transform|BreakTransform (Variables|Default|GetCurrentTransform))))) (Variables|Default|GetBulletSpeed)) (.Y (Math|Vector|BreakVector (.Location (Math|Transform|BreakTransform (Variables|Default|GetCurrentTransform))))) (.Z (Math|Vector|BreakVector (.Location (Math|Transform|BreakTransform (Variables|Default|GetCurrentTransform)))))) (.Rotation (Math|Transform|BreakTransform (Variables|Default|GetCurrentTransform))) (.Scale (Math|Transform|BreakTransform (Variables|Default|GetCurrentTransform))))))

(fn SetBulletColorMaterial
  ;[0.15 0.15 0.15 0.5] Comment
  (bind _returnvalue (Rendering|Material|CreateDynamicMaterialInstance (Variables|Default|GetBullet_Sphere) 0 "/Game/Asset/Material/MI_GridCube.MI_GridCube" "None" :!class /Script/Engine.PrimitiveComponent))
  (Rendering|Material|SetVectorParameterValue _returnvalue "GridColor" (CallFunction|GetLinearColorbyColorType (Variables|Default|GetColorOfBullet)) :!class /Script/Engine.MaterialInstanceDynamic))